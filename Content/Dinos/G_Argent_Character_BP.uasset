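; Argentavis dino character Blueprint that lets the flyer carry creatures in separate beak and claw slots.
; Grabs require flight, a cooldown and optional mass limits, with PvE server rules for dinos.
; Passengers drop on repeat grab attacks, post-attack death, landing (claws only) or rider dismount (humans only).
; Slot state, movement mode and attack multicasts drive the carry montage, while tick animates the feather material by speed.
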(event `MulticastOnAttack`
  (set `self.UpdateCarryAnimAfterAttack` true))

(event `MulticastUpdateCarryAnim`
  (`KismetSystemLibrary.RetriggerableDelay` null 0.25)
  (`self.UpdateCarryAnim`))

(event `self.BSetupDinoTameable`
  (`parent.BSetupDinoTameable`)
  (`/Engine/EditorBlueprintResources/ActorMacros.Switch Has Authority`
    (:`Authority`
      (`self.DeactivateBuffs` (`self.RegenBuffClass`) null))))

(fn `Allow Passenger in Slot`
  (params (Character :type "PrimalCharacter Object Reference") (Slot :type Integer))
  (returns (Allowed :type Boolean))
  (locals (RetVal :type Boolean))
  (bind _mass (`CharacterMovementComponent.Mass` (`Character.CharacterMovement` Character)))
  (set `local.RetVal` false)
  (`|ExecutionSequence`
    (:`then_0`
      (if (and (`|EnumEquality` (`CharacterMovementComponent.MovementMode` (`self.CharacterMovement`)) "MOVE_Flying") (`VictoryCore.IsTimeSince` null (`self.LastGrabTime`) (`self.GetGrabCooldown` Slot)))
        (if (== Slot (`self.ClawsPassengerSlot`))
          (if (or (<= _mass (`self.ClawsCarryMassLimit`)) (not (`self.UseClawsMassLimit`)))
            (set `local.RetVal` true))
          (elif (== Slot (`self.BeakPassengerSlot`))
            (if (or (<= _mass (`self.BeakCarryMassLimit`)) (not (`self.UseBeakMassLimit`)))
              (set `local.RetVal` true))))))
    (:`then_1`
      ;[0 1 0.8594] PVE Servers: Prevent grabbing enemy tames if not allied, and prevent grabbing wild dinos if AllowFlyerCarryPvE is false
      (if (`local.RetVal`)
        (bind _asprimal_dino_character (cast `PrimalDinoCharacter` Character))
        (if (`self.BPIsTamed`)
          (bind _asshooter_game_state (cast `ShooterGameState` (`GameplayStatics.GetGameState` null)))
          (if (`ShooterGameState.bServerPVE` _asshooter_game_state)
            (if (`self.BPIsTamed` _asprimal_dino_character)
              (bind _returnvalue (`self.IsAlliedWithOtherTeam` (`Actor.TargetingTeam` _asprimal_dino_character))) ; In PVE, you cannot carry other player's dinos
              (if (not _returnvalue)
                (set `local.RetVal` false))
              (else
                (bind _asshooter_game_mode (cast `ShooterGameMode` (`GameplayStatics.GetGameMode` null)))
                (bind _returnvalue_2 (`ShooterGameMode.GetBoolOptionIni` _asshooter_game_mode "ServerSettings" "AllowFlyerCarryPvE" false))
                (if (not _returnvalue_2)
                  (set `local.RetVal` false))))))))
    (:`then_2`
      (return (`local.RetVal`)))))

(fn `BlueprintCanRiderAttack`
  (params (AttackIndex :type Integer))
  (returns (ReturnValue :type Boolean))
  (locals (AttackAllowed :type Boolean))
  (bind _clawspassengerslot (`self.ClawsPassengerSlot`))
  (bind _beakpassengerslot (`self.BeakPassengerSlot`))
  (set `local.AttackAllowed` true)
  (`|ExecutionSequence`
    (:`then_0`
      (if (== AttackIndex 0)
        (if (and (`self.Has Passenger In Slot` (`self.ClawsPassengerSlot`)) (`self.Has Passenger In Slot` (`self.BeakPassengerSlot`)))
          (set `local.AttackAllowed` false))
        (elif (== AttackIndex 1)
          (if (`self.Has Passenger In Slot` _clawspassengerslot)
            (`self.Remove Passenger In Slot` _clawspassengerslot)
            (set `local.AttackAllowed` false))
          (elif (== AttackIndex 2)
            (if (`self.Has Passenger In Slot` _beakpassengerslot)
              (`self.Remove Passenger In Slot` _beakpassengerslot)
              (set `local.AttackAllowed` false))))))
    (:`then_1`
      (return (`local.AttackAllowed`)))))

(fn `BPAllowCarryCharacter`
  (params (checkCharacter :type "PrimalCharacter Object Reference"))
  (returns (ReturnValue :type Boolean))
  (bind _allowed (`self.Allow Passenger in Slot` checkCharacter (`self.ClawsPassengerSlot`)))
  (return _allowed))

(fn `BPCanTakePassenger`
  (params (Character :type "PrimalCharacter Object Reference") (PassengerSeatIndex :type Integer) (bForcePassenger :type Boolean) (bAllowFlyersAndWaterDinos :type Boolean))
  (returns (ReturnValue :type Boolean))
  (bind _allowed (`self.Allow Passenger in Slot` Character PassengerSeatIndex))
  (return _allowed))

(fn `BPDidClearCarriedCharacter`
  (params (WithPreviousCarriedCharacter :type "PrimalCharacter Object Reference"))
  (`self.UpdateCarryAnim`))

(fn `BPDoAttack`
  (params (AttackIndex :type Integer))
  (`self.MulticastOnAttack`) ; let the client know to update things
)

(fn `BPNotifyAddPassenger`
  (params (PassengerChar :type "PrimalCharacter Object Reference") (SeatIndex :type Integer))
  (set `self.LastGrabTime` (`KismetSystemLibrary.GetGameTimeInSeconds` null))
  (`self.UpdateCarryAnim`))

(fn `BPNotifyClearPassenger`
  (params (PassengerChar :type "PrimalCharacter Object Reference") (SeatIndex :type Integer))
  (`self.UpdateCarryAnim`))

(fn `BPNotifyClearRider`
  (params (RiderClearing :type "ShooterCharacter Object Reference"))
  (bind _beakpassengerslot (`self.BeakPassengerSlot`))
  (bind _clawspassengerslot (`self.ClawsPassengerSlot`))
  (if (`KismetSystemLibrary.IsServer` null)
    ;[1 1 1] Auto-remove human passengers when the argie's rider dismounts
    (`|ExecutionSequence`
      (:`then_0`
        (cast `ShooterCharacter` (`self.Get Passenger` _beakpassengerslot))
        (`self.Remove Passenger In Slot` _beakpassengerslot))
      (:`then_1`
        (cast `ShooterCharacter` (`self.Get Passenger` _clawspassengerslot))
        (`self.Remove Passenger In Slot` _clawspassengerslot)))))

(fn `BPOnMovementModeChangedNotify`
  (params (PrevMovementMode :type "EMovementMode Enum" :default "MOVE_None") (PreviousCustomMode :type Byte))
  (bind _clawspassengerslot (`self.ClawsPassengerSlot`))
  (bind _movementmode (`CharacterMovementComponent.MovementMode` (`self.CharacterMovement`)))
  (if (`KismetSystemLibrary.IsServer` null)
    (if (and (`|EnumEquality` PrevMovementMode "MOVE_Flying") (or (`|EnumEquality` _movementmode "MOVE_Walking") (`|EnumEquality` _movementmode "MOVE_Falling")))
      (`self.MulticastUpdateCarryAnim`)
      (if (`self.Has Passenger In Slot` _clawspassengerslot)
        (`self.Remove Passenger In Slot` _clawspassengerslot) ; don't allow carrying in claws when on the ground
      ))))

(fn `Get Passenger`
  (params (Slot :type Integer))
  (returns (Char :type "PrimalCharacter Object Reference"))
  (locals (Result :type "PrimalCharacter Object Reference"))
  (bind _beakpassengerslot (`self.BeakPassengerSlot`))
  (`|ExecutionSequence`
    (:`then_0`
      (if (== Slot _beakpassengerslot)
        (set `local.Result` (`self.GetPassengerPerSeat` _beakpassengerslot))
        (elif (== Slot (`self.ClawsPassengerSlot`))
          (set `local.Result` (`self.CarriedCharacter`)))))
    (:`then_1`
      (return (`local.Result`)))))

(fn `Has Passenger In Slot`
  (params (Slot :type Integer))
  (returns (`Return Value` :type Boolean))
  (locals (RetVal :type Boolean))
  (set `local.RetVal` false)
  (`|ExecutionSequence`
    (:`then_0`
      (set `local.RetVal` (`KismetSystemLibrary.IsValid` (`self.Get Passenger` Slot))))
    (:`then_1`
      (return (`local.RetVal`)))))

(fn `ReceiveBeginPlay`
  (bind _returnvalue (`KismetMathLibrary.FMax` (`self.BeakCarryMassLimit`) (`self.ClawsCarryMassLimit`)))
  ;[1 0 0.8203] Make sure the grab weight threshold is enough for both the beak and carry limits
  (if (< (`self.GrabWeightThreshold`) _returnvalue)
    (set `self.GrabWeightThreshold` _returnvalue)))

(fn `ReceiveTick`
  (params (DeltaSeconds :type "Float (single-precision)"))
  (bind _beakpassengerslot (`self.BeakPassengerSlot`))
  (bind _clawspassengerslot (`self.ClawsPassengerSlot`))
  (bind _returnvalue (`self.GetPassengerPerSeat` _clawspassengerslot))
  (bind _returnvalue_2 (`self.GetPassengerPerSeat` _beakpassengerslot))
  (bind _returnvalue_3 (`KismetMathLibrary.FClamp` (/ (`KismetMathLibrary.VSize` (`MovementComponent.Velocity` (`self.CharacterMovement`))) 1000.0)))
  (`|ExecutionSequence`
    (:`then_0`
      ;[1 1 1] Update carry anim after attack ends
      (if (and (not (`KismetSystemLibrary.IsDedicatedServer` null)) (`self.UpdateCarryAnimAfterAttack`))
        (bind _returnvalue_4 (`self.IsCurrentlyPlayingAttackAnimation`))
        (if (not _returnvalue_4)
          (set `self.UpdateCarryAnimAfterAttack` false)
          (`|ExecutionSequence`
            (:`then_0`
              ;[1 1 1] If meleeing a passenger, and that passenger ends up dead, drop them
              (`|ExecutionSequence`
                (:`then_0`
                  (`/Engine/EditorBlueprintResources/StandardMacros.IsValid` _returnvalue_2
                    (:`Is Valid`
                      (if (not (`self.IsAlive` _returnvalue_2))
                        (`self.Remove Passenger In Slot` _beakpassengerslot)))))
                (:`then_1`
                  (`/Engine/EditorBlueprintResources/StandardMacros.IsValid` _returnvalue
                    (:`Is Valid`
                      (if (not (`self.IsAlive` _returnvalue))
                        (`self.Remove Passenger In Slot` _clawspassengerslot)))))))
            (:`then_1`
              (`self.UpdateCarryAnim`))))))
    (:`then_1`
      ;[1 1 1] Keep the feathers material updated based on current movement velocity
      (`/Engine/EditorBlueprintResources/StandardMacros.Can Execute Cosmetic Events`
        (:`True`
          (bind _asmaterial_instance_dynamic (cast `MaterialInstanceDynamic` (`PrimitiveComponent.GetMaterial` (`self.Mesh`) 1)))
          (set `self.FeatherTime` (+ (* DeltaSeconds (`KismetMathLibrary.Lerp` 1.0 3.0 _returnvalue_3)) (`self.FeatherTime`)))
          (`MaterialInstanceDynamic.SetScalarParameterValue` _asmaterial_instance_dynamic "CustomTime" (`self.FeatherTime`))
          (`MaterialInstanceDynamic.SetScalarParameterValue` _asmaterial_instance_dynamic "WindStrength" (`KismetMathLibrary.Lerp` 1.0 2.0 _returnvalue_3)))))))

(fn `Remove Passenger In Slot`
  (params (Slot :type Integer))
  (bind _beakpassengerslot (`self.BeakPassengerSlot`))
  (if (== Slot _beakpassengerslot)
    (`self.RemovePassenger` (`self.Get Passenger` _beakpassengerslot))
    (elif (== Slot (`self.ClawsPassengerSlot`))
      (`self.ClearCarriedCharacter` false))))

(fn `UpdateCarryAnim`
  (locals (NewAnim :type "AnimMontage Object Reference"))
  (bind _beakcarryanim (`self.BeakCarryAnim`))
  (bind _beakcarrygroundanim (`self.BeakCarryGroundAnim`))
  (bind _return_value (`self.Has Passenger In Slot` (`self.BeakPassengerSlot`)))
  (bind _return_value_2 (`self.Has Passenger In Slot` (`self.ClawsPassengerSlot`)))
  (`/Engine/EditorBlueprintResources/StandardMacros.Can Execute Cosmetic Events`
    (:`True`
      (`|ExecutionSequence`
        (:`then_0`
          (set `local.NewAnim` null) ; init to null
        )
        (:`then_1`
          (if (and _return_value_2 _return_value)
            (set `local.NewAnim` (`self.BeakAndClawCarryAnim`))
            (elif _return_value_2
              (set `local.NewAnim` (`self.ClawCarryAnim`))
              (elif _return_value
                (set `local.NewAnim` (select `EMovementMode` (`CharacterMovementComponent.MovementMode` (`self.CharacterMovement`)) :`MOVE_None` _beakcarrygroundanim :`MOVE_Walking` _beakcarrygroundanim :`MOVE_NavWalking` _beakcarrygroundanim :`MOVE_Falling` _beakcarrygroundanim :`MOVE_Swimming` _beakcarryanim :`MOVE_Flying` _beakcarryanim :`MOVE_Custom` _beakcarryanim))))))
        (:`then_2`
          (`self.PlayCarryingMontage` (`local.NewAnim`)))))))

(fn `UserConstructionScript`
  (`parent.UserConstructionScript`))