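; Pteranodon dino character Blueprint that customizes flight movement for its barrel roll boost.
; It intercepts forward input while the barrel roll attack montage plays.
; For a short window after a boost impulse, flying velocity steers toward the last desired rotation under scaled turn-rate limits, with extra speed from the RiderEjectionImpulse magnitude fading linearly down to max speed.
; During that window, desired rotation follows the velocity direction.
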(fn `BP_InterceptMoveForward`
  (params (axisValue :type "Float (single-precision)"))
  (returns (ReturnValue :type Boolean))
  (`|ExecutionSequence`
    (:`then_0`
      (bind _returnvalue (`self.IsCurrentlyPlayingAttackAnimation`))
      (if _returnvalue
        (if (== (`self.GetCurrentMontage`) "/Game/PrimalEarth/Dinos/Ptero/Animations/Ptero-Barrel_Roll_Rit_Montage.Ptero-Barrel_Roll_Rit_Montage")
          (return true))))
    (:`then_1`
      (return false))))

(fn `BPModifyDesiredRotation`
  (params (DeltaTime :type "Float (single-precision)") (InDesiredRotation :type "Rotator Structure (by ref)"))
  (returns (OutDesiredRotation :type "Rotator Structure") (ReturnValue :type Boolean))
  (`|ExecutionSequence`
    (:`then_0`
      (if (`KismetMathLibrary.InRange_FloatFloat` (* (`VictoryCore.TimeSince` null (`self.LastBoostDinoImpulseTime`)) 0.5))
        (return (`KismetMathLibrary.Conv_VectorToRotator` (`self.GetVelocity` false)) true)))
    (:`then_1`
      (return InDesiredRotation false))))

(fn `BPOverrideFlyingVelocity`
  (params (InitialVelocity :type "Vector Structure (by ref)") (Gravity :type "Vector Structure (by ref)") (DeltaTime :type "Float (single-precision)"))
  (returns (ReturnValue :type "Vector Structure"))
  (bind _charactermovement (`self.CharacterMovement`))
  (bind _barrelrollrotationratemultiplier (`self.BarrelRollRotationRateMultiplier`))
  (bind _returnvalue (* (`VictoryCore.TimeSince` null (`self.LastBoostDinoImpulseTime`)) 0.5))
  (`|ExecutionSequence`
    (:`then_0`
      (if (`KismetMathLibrary.InRange_FloatFloat` _returnvalue)
        (bind _returnvalue_2 (`VictoryCore.RotateDirToTargetWithAngleLimits` (`KismetMathLibrary.Normal` InitialVelocity) (`KismetMathLibrary.GetForwardVector` (`self.GetLastMovementDesiredRotation`)) (`KismetMathLibrary.MakeRotator` 0.0 (* DeltaTime (.pitch (`CharacterMovementComponent.RotationRate` _charactermovement)) _barrelrollrotationratemultiplier) (* DeltaTime (.yaw (`CharacterMovementComponent.RotationRate` _charactermovement)) _barrelrollrotationratemultiplier))))
        (return (* _returnvalue_2 (+ (* (- 1.0 (`KismetMathLibrary.FClamp01` _returnvalue)) (`KismetMathLibrary.VSize` (`self.RiderEjectionImpulse`))) (`MovementComponent.GetMaxSpeed` _charactermovement))))))
    (:`then_1`
      (return InitialVelocity))))

(fn `UserConstructionScript`
  (`parent.UserConstructionScript`))