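; Trike dino character with a charged ram attack, bone-based damage reflection and a rivalry buff.
; Ram hold time scales speed, turn rate, damage, impulse and stamina drain, feeding a HUD meter; an anim notify launches it, backed by a timer.
; BPAdjustDamage reflects qualifying hits on configured bones back at attackers, capped.
; A randomized-interval server timer octree-scans for heavy, non-allied carnivores to apply or renew the buff.
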(event `self.ReceiveBeginPlay`
  ;[1 0 0.3281] Rivalry buff checks
  (if (and (`KismetSystemLibrary.IsServer` null) (not (`self.bIsTemporaryMissionDino`)))
    (set `self.RivalryBuffTickInterval` (`KismetMathLibrary.RandomFloatInRange` 4.5 7.0))
    (`KismetSystemLibrary.K2_SetTimerDelegate` (delegate `CheckRivalryTick`) (`self.RivalryBuffTickInterval`) true)))

(event `CheckRivalryTick`
  (bind _returnvalue (`self.GetBuff` (`self.RivalryBuffClass`)))
  ;[1 0 0.3281] Rivalry buff checks
  (`/Engine/EditorBlueprintResources/StandardMacros.IsValid` _returnvalue
    (:`Is Valid`
      (if (<= (- (`PrimalBuff.GetDeactivationTime` _returnvalue) (`KismetSystemLibrary.GetGameTimeInSeconds` null)) (+ (`self.RivalryBuffTickInterval`) 1.0))
        (bind _returnvalue_2 (`VictoryCore.ServerOctreeOverlapActorsClass` null (`self.K2_GetActorLocation`) 5500.0 "DINOPAWNS" "/Script/ShooterGame.PrimalDinoCharacter" true :!label _label))
        (for _array_element _returnvalue_2
          (bind _asprimal_dino_character (cast `PrimalDinoCharacter` _array_element))
          (bind _returnvalue_3 (`self.IsAlliedWithOtherTeam` (`Actor.TargetingTeam` _asprimal_dino_character)))
          (if (and (not _returnvalue_3) (> (`CharacterMovementComponent.Mass` (`Character.CharacterMovement` _asprimal_dino_character)) (`self.RivalryBuffMassThresholdTrigger`)) (`self.IsAlive` _asprimal_dino_character) (`PrimalDinoCharacter.bIsCarnivore` _asprimal_dino_character))
            (`PrimalBuff.StaticAddBuff` (`self.RivalryBuffClass`) self null null)
            (break)))))
    (:`Is Not Valid`
      (goto _label))))

(event `DoReflectDamage`
  (params (DamageTarget :type "Pawn Object Reference") (Damage :type "Float (double-precision)") (BoneName :type Name))
  (bind _returnvalue (`self.K2_GetActorLocation` DamageTarget))
  (bind _returnvalue_2 (`KismetMathLibrary.GetDirectionUnitVector` (`SceneComponent.GetSocketLocation` (`self.Mesh`) "c_head") _returnvalue))
  ;[0.007812 1 0] Damage reflection
  (if (`KismetSystemLibrary.IsServer` null)
    (`GameplayStatics.ApplyPointDamage` DamageTarget (`KismetMathLibrary.FClamp` Damage 0.0 (`self.MaxReflectedDamage`)) _returnvalue_2 (`VictoryCore.MakeHitResult` _returnvalue _returnvalue_2 null DamageTarget (`self.GetPawnRootComponent` DamageTarget) "None" 0 true) (`self.GetController`) self (`self.ReflectedDamageType`) 50000.0)
    (`self.MulticastReflectDamageEffect` BoneName)))

(event `MulticastReflectDamageEffect`
  (params (FromBone :type Name))
  ;[0.007812 1 0] Damage reflection
  (`/Engine/EditorBlueprintResources/StandardMacros.Can Execute Cosmetic Events`
    (:`True`
      (`|SpawnActorFromClass` (`self.DamageReflectionEffect`) (`KismetMathLibrary.Conv_VectorToTransform` (`SceneComponent.GetSocketLocation` (`self.Mesh`) FromBone)) "AlwaysSpawn" "SelectDefaultAtRuntime" null (struct) null))))

(event `RamBuildupEndEvent`
  (`self.Stop Ram Attack Buildup`))

(event `self.BP_OnJumpPressed`
  ;[0.3799 0.6094 1] Space bar cancels any ram
)

(fn `BlueprintAnimNotifyCustomEvent`
  (params (CustomEventName :type Name) (MeshComp :type "SkeletalMeshComponent Object Reference") (Animation :type "AnimSequenceBase Object Reference") (AnimNotifyObject :type "AnimNotify Object Reference"))
  (bind _builduphuffcount (`self.BuildupHuffCount`))
  (bind _returnvalue (`KismetMathLibrary.Conv_IntToDouble` _builduphuffcount))
  (if (== CustomEventName "StartRam")
    (`KismetSystemLibrary.K2_ClearTimer` null "RamBuildUpEndEvent")
    (`self.Stop Ram Attack Buildup`)
    (elif (== CustomEventName "BuildupHuff")
      (set `self.BuildupHuffCount` (+ _builduphuffcount 1))
      (`GameplayStatics.SpawnSoundAttached` "/Game/PrimalEarth/Dinos/Trike/Sounds/Trike_Ram_Loop_Cue.Trike_Ram_Loop_Cue" (`self.Mesh`) "None" (0.0 0.0 0.0) (struct) "KeepRelativeOffset" true (`CurveFloat.GetFloatValue` (`self.BuildupHuffVolume`) _returnvalue) (`CurveFloat.GetFloatValue` (`self.BuildupHuffPitch`) _returnvalue) 0.0 null null))))

(fn `BlueprintCanAttack`
  (params (AttackIndex :type Integer) (distance :type "Float (single-precision)") (attackRangeOffset :type "Float (single-precision)") (OtherTarget :type "Actor Object Reference"))
  (returns (ReturnValue :type Boolean))
  (locals (CanAttack :type Boolean))
  (set `local.CanAttack` (not (`self.RamStarted`)))
  (`|ExecutionSequence`
    (:`then_0`
      (if (and (`local.CanAttack`) (== AttackIndex 1))
        (bind _allowedtoram (`self.CanStartRamAttack`))
        (if (not _allowedtoram)
          (set `local.CanAttack` false))))
    (:`then_1`
      (return (`local.CanAttack`)))))

(fn `BlueprintCanRiderAttack`
  (params (AttackIndex :type Integer))
  (returns (ReturnValue :type Boolean))
  (return (and (!= AttackIndex 1) (not (`self.RamStarted`)))))

(fn `BP_GetCustomModifier_MaxSpeed`
  (returns (ReturnValue :type "Float (single-precision)"))
  (return (`KismetMathLibrary.SelectFloat` (`VictoryCore.SimpleCurveInterpClamped` 1.0 (`self.CalculatedRamMaxSpeed`) (/ (+ (`VictoryCore.TimeSince` null (`self.RamStartTime`)) 0.001) (+ (`self.RamAccelerationTime`) 0.001)) "Linear") 1.0 (`self.RamStarted`))))

(fn `BPAdjustDamage`
  (params (IncomingDamage :type "Float (single-precision)") (TheDamageEvent :type "DamageEvent Structure") (EventInstigator :type "Controller Object Reference") (DamageCauser :type "Actor Object Reference") (bIsPointDamage :type Boolean) (PointHitInfo :type "HitResult Structure"))
  (returns (ReturnValue :type "Float (single-precision)"))
  (locals (ReflectedDamage :type "Float (double-precision)") (BoneName :type Name))
  (bind _returnvalue (`KismetSystemLibrary.IsValid` EventInstigator))
  (bind _returnvalue_2 (`Controller.K2_GetPawn` EventInstigator))
  (bind _reflecteddamage (`local.ReflectedDamage`))
  (set `local.BoneName` "None")
  (set `local.ReflectedDamage` 0.0)
  (if (`self.EnableDamageReflection`)
    (`|ExecutionSequence`
      (:`then_0`
        ;[1 1 1] Figure out if we're reflecting any damage
        (if (and (!= (`VictoryCore.IsChildOfClasses` (`.DamageTypeClass` (break `DamageEvent` TheDamageEvent)) (`self.DamageReflectionTypes`)) -1) _returnvalue)
          (bind _returnvalue_3 (`VictoryCore.GetHitBoneNameFromDamageEvent` self EventInstigator TheDamageEvent bIsPointDamage PointHitInfo))
          (if (and (!= _returnvalue_3 "None") (!= _returnvalue_3 "DinoPawnCapsule"))
            (for _array_element (`self.DamageReflectionBones`)
              (bind (_bonename _damagemultiplier) (break `BoneDamageAdjuster` _array_element))
              (if (== _bonename _returnvalue_3)
                (set `local.ReflectedDamage` (* (`.OriginalDamage` (break `DamageEvent` TheDamageEvent)) _damagemultiplier))
                (set `local.BoneName` _returnvalue_3)
                (break))))))
      (:`then_1`
        ;[1 1 1] Reflect damage back
        (if (and _returnvalue (`KismetSystemLibrary.IsValid` _returnvalue_2) (> _reflecteddamage 0.0))
          (`self.DoReflectDamage` _returnvalue_2 _reflecteddamage (`local.BoneName`))))
      (:`then_2`
        (return IncomingDamage)))
    (else
      (return IncomingDamage))))

(fn `BPGetHUDOverrideBuffProgressBarPercent`
  (returns (ReturnValue :type "Float (single-precision)"))
  (return (`KismetMathLibrary.SelectFloat` (`KismetMathLibrary.FClamp` (/ (`VictoryCore.TimeSince` null (`self.RamBuildupStartTime`)) (`self.RamMaxBuildupTime`))) (`KismetMathLibrary.SelectFloat` (`KismetMathLibrary.MapRangeUnclamped` (/ (- (`self.RamEndTime`) (`KismetSystemLibrary.GetGameTimeInSeconds` null)) (`KismetMathLibrary.FMax` (`self.RamDuration`) 0.001)) 0.0 1.0 0.0 (`self.RamHUDStartPercentage`)) -1.0 (`self.RamStarted`)) (`self.IsRamBuildup`))))

(fn `BPHandleControllerInitiatedAttack`
  (params (AttackIndex :type Integer))
  (returns (ReturnValue :type Boolean))
  (locals (RequestAttack :type Boolean))
  (set `local.RequestAttack` true)
  (`|ExecutionSequence`
    (:`then_0`
      (if (and (>= (- (`KismetSystemLibrary.GetGameTimeInSeconds` null) (`self.RiderLastInitiatedRamTimeSeconds`)) (`.RiderAttackInterval` (break `DinoAttackInfo` (`|GetArrayItem` (`self.AttackInfos`) 1)))) (not (`self.IsSubmerged` false)) (== AttackIndex 1))
        (set `self.RiderLastInitiatedRamTimeSeconds` (`KismetSystemLibrary.GetGameTimeInSeconds` null))
        (`self.Start Ram Attack Buildup`)
        (elif (and (`self.RamStarted`) (== AttackIndex 0) (`VictoryCore.IsTimeSince` null (`self.RamStartTime`) 0.5))
          (`self.ServerRequestRamEndEarly` false)
          (elif (or (`self.RamStarted`) (`self.IsRamBuildup`))
            (set `local.RequestAttack` false)))))
    (:`then_1`
      (return (not (`local.RequestAttack`))) ; return FALSE if we want to request the server to do the attack
    )))

(fn `BPHandleOnStopTargeting`
  (returns (ReturnValue :type Boolean))
  (`self.Stop Ram Attack Buildup`)
  (return true))

(fn `Calculate Ram Duration`
  (params (HoldTime :type "Float (double-precision)"))
  (returns (Duration :type "Float (double-precision)"))
  (return (`KismetMathLibrary.SelectFloat` (* HoldTime 1.5) 20.0 (`self.bHasRider`))))

(fn `CanStartRamAttack`
  (returns (AllowedToRam :type Boolean))
  (return (not (`self.IsSubmerged` false))))

(fn `CanTickStartedRam`
  (returns (tick :type Boolean))
  (return (not false)))

(fn `GetPawnRootComponent`
  (params (target :type "Actor Object Reference"))
  (returns (AsPrimitiveComponent :type "PrimitiveComponent Object Reference"))
  (locals (Comp :type "PrimitiveComponent Object Reference"))
  (set `local.Comp` null)
  (bind _asprimitive_component (cast `PrimitiveComponent` (`self.K2_GetRootComponent` target))
    (:`then`
      (set `local.Comp` _asprimitive_component))
    (:`CastFailed`
      _))
  (return (`local.Comp`)))

(fn `GetRammingSpeedMax`
  (returns (MaxSpeed :type "Float (double-precision)"))
  (return (`self.RammingSpeedMax`)))

(fn `Handle Ram Ended`
  (params (HitSomething :type Boolean))
  (bind _charactermovement (`self.CharacterMovement`))
  (`|ExecutionSequence`
    (:`then_0`
      (if HitSomething
        (`self.PlayAnimEx` (`self.RamOutAnim`) 1.0 "None" true true)))
    (:`then_1`
      (bind _returnvalue (`VictoryCore.GetDefaultObject` self))
      (bind _ascharacter (cast `Character` _returnvalue))
      (bind _charactermovement_2 (`Character.CharacterMovement` _ascharacter))
      (set `CharacterMovementComponent.MaxStepHeight` (`CharacterMovementComponent.MaxStepHeight` _charactermovement_2) _charactermovement) ; restore to default
      (set `CharacterMovementComponent.RotationRate` (`CharacterMovementComponent.RotationRate` _charactermovement_2) _charactermovement)
      (set `self.PlayedRamBuildUpOutAnim` false)
      (`KismetSystemLibrary.K2_ClearTimer` null "RamBuildUpEndEvent"))))

(fn `Handle Ram Started`
  (params (RamBuildupTime :type "Float (double-precision)") (RamDuration :type "Float (double-precision)"))
  (bind _charactermovement (`self.CharacterMovement`))
  (bind _returnvalue (`KismetMathLibrary.FClamp` (/ RamBuildupTime (`self.RamMaxBuildupTime`))))
  (set `self.RamEndTime` (+ (`KismetSystemLibrary.GetGameTimeInSeconds` null) RamDuration)) ; set the ram end time so the progress bar can show time remaining
  (set `CharacterMovementComponent.MaxStepHeight` (`self.MaxStepHeightDuringRam`) _charactermovement)
  (set `CharacterMovementComponent.RotationRate` (`KismetMathLibrary.RLerp` (`self.RotationRateDuringRamMax`) (`self.RotationRateDuringRamMin`) _returnvalue) _charactermovement)
  (set `self.CalculatedRamMaxSpeed` (`VictoryCore.SimpleCurveInterpClamped` (`self.RammingSpeedMin`) (`self.RammingSpeedMax`) _returnvalue "Linear"))
  (set `self.RamDamageDone` (`VictoryCore.SimpleCurveInterpClamped` (`self.RamDamageMin`) (`self.RamDamageMax`) _returnvalue "Linear"))
  (set `self.RamDamageImpulse` (`VictoryCore.SimpleCurveInterpClamped` (`self.RamImpulseMin`) (`self.RamImpulseMax`) _returnvalue "Linear"))
  (set `self.RamStaminaPerSecondDrain` (`VictoryCore.SimpleCurveInterpClamped` (`self.RamStaminaPerSecondDrainMin`) (`self.RamStaminaPerSecondDrainMax`) _returnvalue "Linear"))
  (set `self.RamHUDStartPercentage` (`KismetMathLibrary.FClamp` (/ (`VictoryCore.TimeSince` null (`self.RamBuildupStartTime`)) (`self.RamMaxBuildupTime`)))) ; save the starting hud percent so we can drain the meter back down to zero over the ram duration
)

(fn `Start Ram Attack Buildup`
  (`self.PlayAnimEx` (`self.RamBuildupInAnim`))
  (`parent.Start Ram Attack Buildup`))

(fn `Stop Ram Attack Buildup`
  (if (`self.PlayedRamBuildUpOutAnim`)
    (`parent.Stop Ram Attack Buildup`) ; Actaully start the ram now
    (else
      (bind _returnvalue (`self.PlayAnimEx` (`self.RamBuildupOutAnim`) 1.0 "None" true true))
      (`KismetSystemLibrary.K2_SetTimer` null "RamBuildUpEndEvent" _returnvalue) ; HACK: AnimNotifies don't seem to always trigger for montages that that are so short that they are shorter then their blend in/out times. This will force ram start if the notify doesn't trigger.
      (set `self.PlayedRamBuildUpOutAnim` true)
      (set `self.BuildupHuffCount` 0))))

(fn `UserConstructionScript`
  (`parent.UserConstructionScript`))