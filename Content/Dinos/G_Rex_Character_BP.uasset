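; Rex dino character with a roar attack, also offered as a cooldown-gated multi-use entry for its team.
; The delayed server-side roar filters an octree overlap to a forward cone, making lighter, lower-level hostiles poop and debuffing non-players, with Fortitude raising resistance.
; Rider attack, targeting and FOV hooks forward to any Tek helmet buff, which deactivates when the rider clears.
; Tick disables mesh morph targets when the camera is distant.
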(event `InputAction|GamepadRightThumbstick`
  (params (Key :type "Key Structure"))
  (:`Pressed`
    (for _array_element (`self.GetBuffs`) :!label _label
      (bind _asbuff_dino_tek_helmet_base (cast `/Game/PrimalEarth/CoreBlueprints/Buffs/Buff_DinoTekHelmet_Base` _array_element))
      (`/Game/PrimalEarth/CoreBlueprints/Buffs/Buff_DinoTekHelmet_Base.PressedAltFire` _asbuff_dino_tek_helmet_base)
      (break))))

(event `InputAction|AltFire`
  (params (Key :type "Key Structure"))
  (:`Pressed`
    (goto _label)))

(event `RoarCameraShake`
  (`KismetSystemLibrary.Delay` null (`self.RoarCameraShake_StartDelay`))
  (bind _returnvalue (`Controller.CastToPlayerController` (`self.GetController`)))
  (`PlayerController.ClientStartCameraShake` :`self` _returnvalue :`Shake` "/Game/ScorchedEarth/Dinos/Manticore/ManticoreRoar_CameraShake.ManticoreRoar_CameraShake_C" :`Scale` (`self.RoarCameraShake_Scale`) :`Speed` (`self.RoarCameraShake_Speed`)))

(event `DoRoarOverlapsAfterDelay`
  (if (`KismetSystemLibrary.IsServer` null)
    (`KismetSystemLibrary.Delay` null (`self.RoarCameraShake_StartDelay`))
    (`self.Roar`)))

(event `self.ReceiveTick`
  (params (DeltaSeconds :type "Float (single-precision)"))
  (bind _mesh (`self.Mesh`))
  (bind _returnvalue (not (`SkinnedMeshComponent.bDisableMorphTarget` (`self.Mesh`))))
  ;[0 0.3906 1] Disable Morph Target at a distance
  (bind _asshooter_player_controller (cast `ShooterPlayerController` (`GameplayStatics.GetPlayerController` null)))
  (if (< (`KismetMathLibrary.VSize` (- (`self.K2_GetActorLocation`) (`PlayerCameraManager.GetCameraLocation` (`PlayerController.PlayerCameraManager` _asshooter_player_controller)))) 2000.0)
    (if (not _returnvalue)
      (set `SkinnedMeshComponent.bDisableMorphTarget` false _mesh))
    (elif _returnvalue
      (set `SkinnedMeshComponent.bDisableMorphTarget` true _mesh))))

(fn `AllowRoarStun`
  (params (primalChar :type "PrimalCharacter Object Reference"))
  (returns (result :type Boolean))
  (locals (retVal :type Boolean) (AdditionalFortitudeLevel :type Integer))
  (bind _mycharacterstatuscomponent (`PrimalCharacter.MyCharacterStatusComponent` primalChar))
  (bind _mycharacterstatuscomponent_2 (`self.MyCharacterStatusComponent`))
  (bind _bdebugrex (`self.bDebugRex`))
  (bind _returnvalue (`KismetStringLibrary.Concat_StrStr` (`KismetSystemLibrary.GetDisplayName` primalChar) " :: "))
  (bind _returnvalue_2 (+ (`PrimalCharacterStatusComponent.BaseCharacterLevel` _mycharacterstatuscomponent_2) (`PrimalCharacterStatusComponent.GetExtraCharacterLevel` _mycharacterstatuscomponent_2)))
  (bind _returnvalue_3 (+ (`PrimalCharacterStatusComponent.BaseCharacterLevel` _mycharacterstatuscomponent) (`PrimalCharacterStatusComponent.GetExtraCharacterLevel` _mycharacterstatuscomponent) (`local.AdditionalFortitudeLevel`)))
  (set `local.retVal` false)
  (`|ExecutionSequence`
    (:`then_0`
      (if (!= primalChar self)
        (if (<= (`PrimalCharacter.DragWeight` primalChar) (`self.GrabWeightThreshold`))
          (set `local.AdditionalFortitudeLevel` 0)
          (`|ExecutionSequence`
            (:`then_0`
              (bind _asshooter_character (cast `ShooterCharacter` primalChar)
                (:`then`
                  (bind _returnvalue_4 (`self.GetCharacterStatusComponent` _asshooter_character))
                  (set `local.AdditionalFortitudeLevel` (* (`KismetMathLibrary.FFloor` (`PrimalCharacterStatusComponent.BPGetCurrentStatusValue` _returnvalue_4 "TemperatureFortitude")) (`self.FortitudeLevelScale_Player`))))
                (:`CastFailed`
                  (bind _asprimal_dino_character (cast `PrimalDinoCharacter` primalChar))
                  (if (`PrimalDinoCharacter.bHasRider` _asprimal_dino_character)
                    (bind _returnvalue_5 (`self.GetCharacterStatusComponent` (`PrimalDinoCharacter.Rider` _asprimal_dino_character)))
                    (set `local.AdditionalFortitudeLevel` (* (`self.FortitudeLevelScale_RiddenDino`) (`KismetMathLibrary.FFloor` (`PrimalCharacterStatusComponent.BPGetCurrentStatusValue` _returnvalue_5 "TemperatureFortitude"))))))))
            (:`then_1`
              (if (> _returnvalue_2 _returnvalue_3)
                (if (not (`self.HasBuff` primalChar (`self.PreventRoarBuff`) false))
                  (if (`self.IsHostileTo` primalChar)
                    (set `local.retVal` true)
                    (else
                      (`KismetSystemLibrary.PrintString` null (`KismetStringLibrary.Concat_StrStr` _returnvalue "IGNORED (FRIENDLY)") _bdebugrex _bdebugrex (struct :`R` 1.0 :`G` 0.456137 :`A` 1.0))))
                  (else
                    (`KismetSystemLibrary.PrintString` null (`KismetStringLibrary.Concat_StrStr` _returnvalue "IGNORED (ON COOLDOWN)") _bdebugrex _bdebugrex (struct :`R` 1.0 :`G` 0.456137 :`A` 1.0))))
                (else
                  (`KismetSystemLibrary.PrintString` null (`KismetStringLibrary.Concat_StrStr` _returnvalue (`KismetStringLibrary.BuildString_Int` "IGNORED (OVER LEVEL LIMIT - " (`KismetStringLibrary.Concat_StrStr` (`KismetStringLibrary.Conv_IntToString` _returnvalue_2) " vs ") _returnvalue_3 ")")) _bdebugrex _bdebugrex (struct :`R` 1.0 :`G` 0.456137 :`A` 1.0))))))
          (else
            (`KismetSystemLibrary.PrintString` null (`KismetStringLibrary.Concat_StrStr` _returnvalue "IGNORED (OVER DRAG WEIGHT)") _bdebugrex _bdebugrex (struct :`R` 1.0 :`G` 0.456137 :`A` 1.0))))))
    (:`then_1`
      (return (`local.retVal`)))))

(fn `BPDoAttack`
  (params (AttackIndex :type Integer))
  (if (== AttackIndex 1)
    (`self.DoRoarOverlapsAfterDelay`)))

(fn `BPGetMultiUseEntries`
  (params (ForPC :type "PlayerController Object Reference") (MultiUseEntries :type "Array of MultiUseEntry Structure (by ref)"))
  (returns (ReturnValue :type "Array of MultiUseEntry Structure"))
  (bind (_childstateindexes _meleeswingsockets _attackanimations _attackanimationweights _attackanimationstimefromendtoconsiderfinished _lastsocketpositions _attackanimdamageimpactfxsocketnames _attackrotationrate _attackname _rangedsocket _meleedamagetype _projectileclass _attackstatetypeclass _attackstatetype _lastattacktime _riderlastattacktime _attackselectiontime _lastprojectilespawntime _attackweight _attackrange _minattackrange _activateattackrange _attackinterval _attackwithjumpchance _attackselectionexpirationtime _attackrotationrangedegrees _attackrotationgroundspeedmultiplier _meleedamageimpulse _meleeswingradius _attackoffset _staminacost _riderattackinterval) (break `DinoAttackInfo` (`|GetArrayItem` (`self.AttackInfos`) 1)))
  (`|ExecutionSequence`
    (:`then_0`
      (if (and (`self.BPIsConscious`) (not (`self.IsBaby`)))
        (if (== (`Actor.TargetingTeam` ForPC) (`self.TargetingTeam`))
          (bind _asshooter_game_state (cast `ShooterGameState` (`GameplayStatics.GetGameState` null)))
          (bind _returnvalue (`ShooterGameState.GetNetworkTimeDelta` _asshooter_game_state (`self.lastTamedRoarTime`) false))
          (bind _returnvalue_2 (`self.CanAttack` 1))
          (bind _returnvalue_3 (`KismetStringLibrary.Conv_DoubleToString` (- _riderattackinterval _returnvalue)))
          (bind _returnvalue_4 (< _returnvalue _riderattackinterval))
          (`KismetArrayLibrary.Array_Add` MultiUseEntries (make `MultiUseEntry` null (`KismetMathLibrary.SelectString` (`KismetStringLibrary.BuildString_Name` "" "Roar (" (`KismetStringLibrary.Conv_StringToName` (`KismetStringLibrary.GetSubstring` _returnvalue_3 0 (+ (`KismetStringLibrary.FindSubstring` _returnvalue_3 "." false true) 2))) ")") "Roar" _returnvalue_4) (`self.RoarMultiUseIndex`) -999999999 false (or (not _returnvalue_2) _returnvalue_4) false false false false false false false true false false false false null false 0 (struct :`B` 175 :`G` 175 :`R` 175 :`A` 255) (`KismetMathLibrary.Conv_LinearColorToColor` (make `LinearColor` 1.0 0.5 0.0 1.0)) 0.0 0.0 null -1 -1 (`self.Icon_Roar`))))))
    (:`then_1`
      (return MultiUseEntries))))

(fn `BPHandleControllerInitiatedAttack`
  (params (AttackIndex :type Integer))
  (returns (ReturnValue :type Boolean))
  (locals (retVal :type Boolean))
  (`|ExecutionSequence`
    (:`then_0`
      (for _array_element (`self.GetBuffs`)
        (bind _asbuff_dino_tek_helmet_base (cast `/Game/PrimalEarth/CoreBlueprints/Buffs/Buff_DinoTekHelmet_Base` _array_element))
        (if (== AttackIndex 0)
          (bind _bdidattack (`/Game/PrimalEarth/CoreBlueprints/Buffs/Buff_DinoTekHelmet_Base.LocalDoAttack` _asbuff_dino_tek_helmet_base))
          (set `local.retVal` _bdidattack)
          (break)
          (elif (== AttackIndex 1)
            (`/Game/PrimalEarth/CoreBlueprints/Buffs/Buff_DinoTekHelmet_Base.SetTargeting` _asbuff_dino_tek_helmet_base true)
            (set `local.retVal` (`/Game/PrimalEarth/CoreBlueprints/Buffs/Buff_DinoTekHelmet_Base.bIsTargetingModeEnabled` _asbuff_dino_tek_helmet_base))
            (break)
            (else
              (break))))))
    (:`then_1`
      (return (`local.retVal`)))))

(fn `BPHandleOnStopTargeting`
  (returns (ReturnValue :type Boolean))
  (for _array_element (`self.GetBuffs`)
    (bind _asbuff_dino_tek_helmet_base (cast `/Game/PrimalEarth/CoreBlueprints/Buffs/Buff_DinoTekHelmet_Base` _array_element))
    (`/Game/PrimalEarth/CoreBlueprints/Buffs/Buff_DinoTekHelmet_Base.SetTargeting` _asbuff_dino_tek_helmet_base false)
    (break))
  (return false))

(fn `BPModifyFOV`
  (params (FOVIn :type "Float (single-precision)"))
  (returns (ReturnValue :type "Float (single-precision)"))
  (locals (retVal :type "Float (double-precision)"))
  (set `local.retVal` FOVIn)
  (`|ExecutionSequence`
    (:`then_0`
      (for _array_element (`self.GetBuffs`)
        (bind _asbuff_dino_tek_helmet_base (cast `/Game/PrimalEarth/CoreBlueprints/Buffs/Buff_DinoTekHelmet_Base` _array_element))
        (if (`/Game/PrimalEarth/CoreBlueprints/Buffs/Buff_DinoTekHelmet_Base.bIsTargetingModeEnabled` _asbuff_dino_tek_helmet_base)
          (set `local.retVal` 55.0)
          (break)
          (else
            (break)))))
    (:`then_1`
      (return (`local.retVal`)))))

(fn `BPNotifyClearRider`
  (params (RiderClearing :type "ShooterCharacter Object Reference"))
  (set `self.bMeleeSwingDamageBlockedByStrutures` true)
  (for _array_element (`self.GetBuffs`)
    (bind _asbuff_dino_tek_helmet_base (cast `/Game/PrimalEarth/CoreBlueprints/Buffs/Buff_DinoTekHelmet_Base` _array_element))
    (if (`/Game/PrimalEarth/CoreBlueprints/Buffs/Buff_DinoTekHelmet_Base.bHelmetActivated` _asbuff_dino_tek_helmet_base)
      (`/Game/PrimalEarth/CoreBlueprints/Buffs/Buff_DinoTekHelmet_Base.DeactivateHelmet` _asbuff_dino_tek_helmet_base))))

(fn `BPNotifySetRider`
  (params (RiderSetting :type "ShooterCharacter Object Reference")))

(fn `BPTryMultiUse`
  (params (ForPC :type "PlayerController Object Reference") (UseIndex :type Integer))
  (returns (ReturnValue :type Boolean))
  (locals (retVal :type Boolean))
  (set `local.retVal` true)
  (`|ExecutionSequence`
    (:`then_0`
      (if (== UseIndex (`self.RoarMultiUseIndex`))
        (set `local.retVal` false)
        (if (== (`Actor.TargetingTeam` ForPC) (`self.TargetingTeam`))
          (bind _returnvalue (`self.CanAttack` 1))
          (if (and _returnvalue (`VictoryCore.IsTimeSince` null (`self.lastTamedRoarTime`) (`.RiderAttackInterval` (break `DinoAttackInfo` (`|GetArrayItem` (`self.AttackInfos`) 1)))))
            (bind _returnvalue_2 (`self.DoAttack` 1 true))
            (set `local.retVal` _returnvalue_2)))))
    (:`then_1`
      (return (`local.retVal`)))))

(fn `GetSocketForMeleeTraceForHitBlockers`
  (params (AttackIndex :type Integer))
  (returns (ReturnValue :type Name))
  (locals (Ret :type Name))
  (`|ExecutionSequence`
    (:`then_0`
      (switch `int` AttackIndex
        (:`0`
          (set `local.Ret` "buffsocketcenterdynamic"))))
    (:`then_1`
      (return (`local.Ret`)))))

(fn `Roar`
  (bind _bdebugrex (`self.bDebugRex`))
  (bind _roarradius (`self.RoarRadius`))
  (bind _location (.location (`SceneComponent.GetSocketTransform` (`self.Mesh`) (`self.RoarOverlapSocket`) "RTS_World")))
  (bind _returnvalue (`KismetMathLibrary.GetForwardVector` (.rotation (`SceneComponent.GetSocketTransform` (`self.Mesh`) (`self.RoarOverlapSocket`) "RTS_World"))))
  (if (`KismetSystemLibrary.IsServer` null)
    (`|ExecutionSequence`
      (:`then_0`
        (bind _returnvalue_2 (`VictoryCore.ServerOctreeOverlapActors` null _location _roarradius "PAWNS"))
        (`|ExecutionSequence`
          (:`then_0`
            (for _array_element _returnvalue_2
              (bind _asprimal_character (cast `PrimalCharacter` _array_element))
              (if (>= (`KismetMathLibrary.Dot_VectorVector` (`KismetMathLibrary.Normal` (- (`self.K2_GetActorLocation` _asprimal_character) _location)) _returnvalue) (`self.Roar_DotProductThreshold`))
                (bind _result (`self.AllowRoarStun` _asprimal_character))
                (if _result
                  (cast `ShooterCharacter` _asprimal_character
                    (:`then`
                      _)
                    (:`CastFailed`
                      (`PrimalBuff.StaticAddBuff` (`self.RoarBuffClass`) _asprimal_character null self)))
                  (`self.Poop` _asprimal_character true)
                  (`KismetSystemLibrary.PrintString` null (`KismetStringLibrary.Concat_StrStr` (`KismetStringLibrary.Concat_StrStr` (`KismetSystemLibrary.GetDisplayName` _asprimal_character) " :: ") "POOP STUNNED") _bdebugrex _bdebugrex (struct :`G` 1.0 :`B` 0.000452 :`A` 1.0))))))
          (:`then_1`
            (if _bdebugrex
              (`KismetSystemLibrary.DrawDebugConeInDegrees` null _location _returnvalue _roarradius 80.0 80.0 30 (struct :`R` 0.986231 :`B` 1.0 :`A` 1.0) 10.0)))))
      (:`then_1`
        (if (`self.bHasRider`)
          (`self.RoarCameraShake`)))
      (:`then_2`
        (if (`self.BPIsTamed`)
          (set `self.lastTamedRoarTime` (`KismetSystemLibrary.GetGameTimeInSeconds` null) true))))))

(fn `UserConstructionScript`
  (`parent.UserConstructionScript`))