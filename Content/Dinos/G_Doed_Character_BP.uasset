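; Doedicurus dino character Blueprint that customizes attack gating, charge movement, charge audio and the low-health animation.
; Attack 0 requires walking or swimming; in other movement modes a rider's attack 0 input triggers attack 2 when available.
; Charging forces full forward acceleration, and its end notify stops the ball-roll loop sound off dedicated servers.
; YutyFear forced exit disables the low-health animation; restore re-enables it from class-default thresholds.
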(event `AnimNotify_EndCharge`
  (if (not (`KismetSystemLibrary.IsDedicatedServer` null))
    (`SceneComponent.StopSound` (`self.K2_GetRootComponent`) "/Game/PrimalEarth/Sound/SFX/Dinos/Doed/Ark_Doedicurus_Ball_Roll_Loop_Cue.Ark_Doedicurus_Ball_Roll_Loop_Cue" 0.3)
    (`SceneComponent.StopSound` (`self.Mesh`) "/Game/PrimalEarth/Sound/SFX/Dinos/Doed/Ark_Doedicurus_Ball_Roll_Loop_Cue.Ark_Doedicurus_Ball_Roll_Loop_Cue" 0.3)))

(event `Multi_ToggleEnableLowHealthAnim`
  (params (Enable :type Boolean))
  (if Enable
    (bind _returnvalue (`VictoryCore.GetDefaultObject` self))
    (bind _asprimal_dino_character (cast `PrimalDinoCharacter` _returnvalue))
    (set `self.LeavePlayAnimBelowHealthPercent` (`PrimalDinoCharacter.LeavePlayAnimBelowHealthPercent` _asprimal_dino_character))
    (set `self.PlayAnimBelowHealthPercent` (`PrimalDinoCharacter.PlayAnimBelowHealthPercent` _asprimal_dino_character))
    (else
      (set `self.LeavePlayAnimBelowHealthPercent` 0.0)
      (set `self.PlayAnimBelowHealthPercent` 0.0)
      (set `self.bIsPlayingLowHealthAnim` false))))

(fn `BlueprintCanAttack`
  (params (AttackIndex :type Integer) (distance :type "Float (single-precision)") (attackRangeOffset :type "Float (single-precision)") (OtherTarget :type "Actor Object Reference"))
  (returns (ReturnValue :type Boolean))
  (locals (canAttack :type Boolean))
  (bind _charactermovement (`self.CharacterMovement`))
  (bind _movementmode (`CharacterMovementComponent.MovementMode` _charactermovement))
  (set `local.canAttack` false)
  (`|ExecutionSequence`
    (:`then_0`
      (if (== AttackIndex 0)
        (if (`KismetSystemLibrary.IsValid` _charactermovement)
          (if (or (`|EnumEquality` _movementmode "MOVE_Walking") (`|EnumEquality` _movementmode "MOVE_Swimming"))
            (bind _returnvalue (`self.CanAttack` 0))
            (set `local.canAttack` _returnvalue)))))
    (:`then_1`
      (return (`local.canAttack`)))))

(fn `BlueprintCanRiderAttack`
  (params (AttackIndex :type Integer))
  (returns (ReturnValue :type Boolean))
  (locals (canDoAttack :type Boolean))
  (bind _charactermovement (`self.CharacterMovement`))
  (bind _movementmode (`CharacterMovementComponent.MovementMode` _charactermovement))
  (set `local.canDoAttack` false)
  (`|ExecutionSequence`
    (:`then_0`
      (if (== AttackIndex 0)
        (if (`KismetSystemLibrary.IsValid` _charactermovement)
          (if (or (`|EnumEquality` _movementmode "MOVE_Swimming") (`|EnumEquality` _movementmode "MOVE_Walking"))
            (bind _returnvalue (`self.CanAttack` 0))
            (set `local.canDoAttack` _returnvalue)
            (else
              (bind _returnvalue_2 (`self.CanAttack` 2))
              (if _returnvalue_2
                (`self.DoAttack` 2 true)))))))
    (:`then_1`
      (return (`local.canDoAttack`)))))

(fn `BPChargingModifyInputAcceleration`
  (params (inputAcceleration :type "Vector Structure"))
  (returns (ReturnValue :type "Vector Structure"))
  (bind _charactermovement (`self.CharacterMovement`))
  (return (* (`SceneComponent.GetForwardVector` (`MovementComponent.UpdatedComponent` _charactermovement)) (`CharacterMovementComponent.MaxAcceleration` _charactermovement))))

(fn `BPForceDinoExitCustomState`
  (params (TypeTag :type Name))
  (if (== TypeTag "YutyFear")
    (`self.Multi_ToggleEnableLowHealthAnim` false)))

(fn `BPRestoreDinoCustomState`
  (params (TypeTag :type Name))
  (if (== TypeTag "YutyFear")
    (`self.Multi_ToggleEnableLowHealthAnim` true)))

(fn `UserConstructionScript`
  (`parent.UserConstructionScript`))