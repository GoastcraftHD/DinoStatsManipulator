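; Base dino character Blueprint that supplies shared creature behavior for impact FX, death, camera and interaction.
; Attacker impact FX take blood color from the victim's hurt decal name and size from the smaller creature.
; Dedicated servers skip death montages to a paused end, while clients hand large footprint FX to temporary actors on stasis or destruction.
; Camera overrides mostly delegate to shared functions, right shoulder reaches buffs, and harness-saddled tames get a consumables auto-transfer toggle.
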(event `self.BPSpawnAttackerDamageImpactFX`
  (params (SocketName :type Name) (VictimChar :type "PrimalCharacter Object Reference"))
  (bind _damageimpactfxsizeoverride (`PrimalCharacter.DamageImpactFXSizeOverride` VictimChar))
  (bind _damageimpactfxsizeoverride_2 (`self.DamageImpactFXSizeOverride`))
  (bind _damageimpactfxforattacker (`PrimalCharacter.DamageImpactFXForAttacker` VictimChar))
  (`/Engine/EditorBlueprintResources/StandardMacros.IsValid` _damageimpactfxforattacker
    (:`Is Valid`
      (bind _returnvalue (`self.GetFXBloodColor` VictimChar))
      (bind _returnvalue_2 (`NiagaraFunctionLibrary.SpawnSystemAttached` _damageimpactfxforattacker (`self.Mesh`) SocketName (0.0 0.0 0.0) (struct) "SnapToTarget" true))
      (`/Engine/EditorBlueprintResources/StandardMacros.IsValid` _returnvalue_2
        (:`Is Valid`
          (`NiagaraComponent.SetVariableLinearColor` _returnvalue_2 "Blood Color" _returnvalue)
          (`NiagaraComponent.SetVariableFloat` _returnvalue_2 "Impact Size" (`KismetMathLibrary.FMin` (`KismetMathLibrary.SelectFloat` _damageimpactfxsizeoverride (`PrimalCharacter.DragWeight` VictimChar) (> _damageimpactfxsizeoverride 0.0)) (`KismetMathLibrary.SelectFloat` _damageimpactfxsizeoverride_2 (`self.DragWeight`) (> _damageimpactfxsizeoverride_2 0.0))))
          (`NiagaraComponent.SetVariableVec3` _returnvalue_2 "Dino Velocity" (`self.GetVelocity` false)))))))

(event `self.BlendSpaceGenerated`
  (params (blendSpace :type "BlendSpace Object Reference"))
  (bind _returnvalue (`KismetSystemLibrary.GetObjectName` blendSpace))
  (if (`KismetSystemLibrary.IsValid` blendSpace)
    (if (`KismetStringLibrary.Contains` _returnvalue "Swim_Idle_Death")
      _
      (elif (`KismetStringLibrary.Contains` _returnvalue "Move_Fwd_Death")
        _
        (elif (`KismetStringLibrary.Contains` _returnvalue "Falling_Death")
          _
          (elif (`KismetStringLibrary.Contains` _returnvalue "Torpid_Death")
            _
            (elif (`KismetStringLibrary.Contains` _returnvalue "Idle_Death")
              _)))))))

(event `self.ReceiveBeginPlay`
  (`parent.ReceiveBeginPlay`))

(event `self.EditorBeginPlay`
  (bind _returnvalue (`VictoryCore.TimeSeconds` null))
  (if (`KismetSystemLibrary.IsDedicatedServer` null)
    (`parent.EditorBeginPlay`)
    (if (`self.bCheatForceTameRide`)
      (if (> (- _returnvalue (`KismetMathLibrary.SelectFloat` 100000000.0 0.0 (> _returnvalue 0.0))) 5.0)
        (if (not (`self.GeneratedBlendSpaces`))
          (bind _returnvalue_2 (`VictoryCore.GetClassDefaultObject` (`GameplayStatics.GetObjectClass` self)))
          (bind _asg_dino_character_bp (cast `/Game/Dinos/G_Dino_Character_BP` _returnvalue_2))
          (set `/Game/Dinos/G_Dino_Character_BP.GeneratedBlendSpaces` true _asg_dino_character_bp)
          (`VictoryCore.GenerateDeathBlendSpacesForDino` self)
          (`/Engine/EditorBlueprintResources/ActorMacros.SwitchNetAuthority`
            (:`DedicatedServer`
              _)
            (:`PlayerServer`
              _))
          (bind _asshooter_game_mode (cast `ShooterGameMode` (`GameplayStatics.GetGameMode` null)))
          (bind _returnvalue_3 (`ShooterGameMode.GetBoolOptionIni` _asshooter_game_mode "DinoStatsManipulator" "RemoveHunger" true))
          (set `self.RemoveHunger` _returnvalue_3)
          (bind _returnvalue_4 (`ShooterGameMode.GetBoolOptionIni` _asshooter_game_mode "DinoStatsManipulator" "RemoveOxygen" true))
          (set `self.RemoveOxygen` _returnvalue_4))))
    (else
      (set `self.bTriggerBPStasis` true))))

(event `self.BP_OnSetDeath`
  ;[1 0 0.2109] Force End and pause on death animation on dedicated server - michaelb
  (`parent.BP_OnSetDeath`)
  (if (`KismetSystemLibrary.IsDedicatedServer` null)
    (`KismetSystemLibrary.DelayUntilNextTick` null)
    (`self.PlayAnimMontage` (`self.GetCurrentMontage`) 1.0 "ForceEndAndPause" true true 0.01 1.0)))

(event `self.BPTriggerStasisEvent`
  (if (`KismetSystemLibrary.IsDedicatedServer` null)
    _
    (elif (`self.DoesUseHibernation`)
      (for _array_element (`self.GetComponentsByTag` "/Script/Engine.SceneComponent" "footprint_fx") :!label _label
        (bind _asscene_component (cast `SceneComponent` _array_element))
        (if (> (`.SphereRadius` (`KismetSystemLibrary.GetComponentBounds` _asscene_component)) 550.0)
          (`SceneComponent.K2_DetachFromComponent` _asscene_component "KeepWorld" "KeepWorld" "KeepWorld" false)
          (bind _returnvalue (`|SpawnActorFromClass` "/Script/Engine.Actor" (`SceneComponent.K2_GetComponentToWorld` _asscene_component) "AlwaysSpawn" "MultiplyWithRoot" null null))
          (`ActorComponent.SetOwner` _asscene_component _returnvalue)
          (`self.SetLifeSpan` _returnvalue (`self.PostDestructionFootstepLifespan`)))))))

(event `self.ReceiveDestroyed`
  (if (not (`KismetSystemLibrary.IsDedicatedServer` null))
    (goto _label)))

(fn `BPControlRigNotify`
  (params (NotifyName :type Name) (NotifyCustomTag :type Name) (WorldSpaceHitResult :type "HitResult Structure (by ref)") (Velocity :type "Vector Structure (by ref)"))
  (`/Game/PrimalEarth/Effects/FL_ControlRigFX.ControlRigNotify` NotifyName NotifyCustomTag WorldSpaceHitResult self)
  (return))

(fn `BPGetMultiUseEntries`
  (params (ForPC :type "PlayerController Object Reference") (MultiUseEntries :type "Array of MultiUseEntry Structure (by ref)"))
  (returns (ReturnValue :type "Array of MultiUseEntry Structure"))
  (bind _supportsconsumablesautotransfer (`self.SupportsConsumablesAutoTransfer`))
  (`|ExecutionSequence`
    (:`then_0`
      (bind _returnvalue (`PrimalAssets.ClassAssetResolve` (`self.HarnesSaddleItem`)))
      (if (and (== (`Actor.TargetingTeam` ForPC) (`self.TamingTeamID`)) (`PrimalInventoryComponent.HasItemsEquipped` (`self.MyInventoryComponent`) (`|MakeArray` _returnvalue) true false true))
        (`KismetArrayLibrary.Array_Add` MultiUseEntries (make `MultiUseEntry` null (`KismetMathLibrary.SelectString` (`KismetTextLibrary.Conv_TextToString` (`self.DisableConsumablesTransferText`)) (`KismetTextLibrary.Conv_TextToString` (`self.EnableConsumablesTransferText`)) _supportsconsumablesautotransfer) 111115 -1000 false false false false false false false false false true false false false false null false 0 (struct :`B` 175 :`G` 175 :`R` 175 :`A` 255) (struct :`B` 255 :`G` 255 :`R` 255 :`A` 255) 0.0 0.0 null -1 -1 (select `bool` _supportsconsumablesautotransfer :`false` "/Game/PrimalEarth/UI/UI_Final_Assets/RW/Structure/RW_Transfer_to_Trough_on.RW_Transfer_to_Trough_on" :`true` "/Game/PrimalEarth/UI/UI_Final_Assets/RW/Structure/RW_Transfer_to_Trough_off.RW_Transfer_to_Trough_off" :!type "Texture2D Object Reference")))))
    (:`then_1`
      (return MultiUseEntries))))

(fn `BPGetRidingMultiUseEntries`
  (params (ForPC :type "PlayerController Object Reference") (MultiUseEntries :type "Array of MultiUseEntry Structure (by ref)"))
  (returns (ReturnValue :type "Array of MultiUseEntry Structure"))
  (bind _supportsconsumablesautotransfer (`self.SupportsConsumablesAutoTransfer`))
  (`|ExecutionSequence`
    (:`then_0`
      (bind _returnvalue (`PrimalAssets.ClassAssetResolve` (`self.HarnesSaddleItem`)))
      (if (and (== (`Actor.TargetingTeam` ForPC) (`self.TamingTeamID`)) (`PrimalInventoryComponent.HasItemsEquipped` (`self.MyInventoryComponent`) (`|MakeArray` _returnvalue) true false true))
        (`KismetArrayLibrary.Array_Add` MultiUseEntries (make `MultiUseEntry` null (`KismetMathLibrary.SelectString` (`KismetTextLibrary.Conv_TextToString` (`self.DisableConsumablesTransferText`)) (`KismetTextLibrary.Conv_TextToString` (`self.EnableConsumablesTransferText`)) _supportsconsumablesautotransfer) 111115 -1000 false false false false false false false false false true false false false false null false 0 (struct :`B` 175 :`G` 175 :`R` 175 :`A` 255) (struct :`B` 255 :`G` 255 :`R` 255 :`A` 255) 0.0 0.0 null -1 -1 (select `bool` _supportsconsumablesautotransfer :`false` "/Game/PrimalEarth/UI/UI_Final_Assets/RW/Structure/RW_Transfer_to_Trough_on.RW_Transfer_to_Trough_on" :`true` "/Game/PrimalEarth/UI/UI_Final_Assets/RW/Structure/RW_Transfer_to_Trough_off.RW_Transfer_to_Trough_off" :!type "Texture2D Object Reference")))))
    (:`then_1`
      (return MultiUseEntries))))

(fn `BPHandleRightShoulderButton`
  (returns (ReturnValue :type Boolean))
  (`|ExecutionSequence`
    (:`then_0`
      (for _array_element (`self.GetBuffs`)
        (bind _asbuff_base (cast `/Game/PrimalEarth/CoreBlueprints/Buffs/Buff_Base` _array_element))
        (`/Game/PrimalEarth/CoreBlueprints/Buffs/Buff_DinoTekHelmet_Base.PressedAltFire` _asbuff_base)
        (return true)))
    (:`then_1`
      (return false))))

(fn `BPOverrideCameraArmLength`
  (params (CameraParams :type "PrimalCameraParams Structure (by ref)") (CurrentCameraArmLength :type "Float (single-precision)") (DesiredCameraArmLength :type "Float (single-precision) (by ref)"))
  (returns (ReturnValue :type Boolean))
  (`|ExecutionSequence`
    (:`then_0`
      (`/Game/PrimalEarth/CoreBlueprints/BPFunctionLibraries/ASACameraFunctionLibrary.FinalOverrideCameraArmLength` self CameraParams self CurrentCameraArmLength DesiredCameraArmLength))
    (:`then_1`
      (return true))))

(fn `BPOverrideCameraArmLengthInterpParams`
  (params (CameraParams :type "PrimalCameraParams Structure (by ref)") (OutInterpParams :type "PrimalCameraInterpParams Structure (by ref)"))
  (returns (ReturnValue :type Boolean))
  (`|ExecutionSequence`
    (:`then_0`
      (`/Game/PrimalEarth/CoreBlueprints/BPFunctionLibraries/ASACameraFunctionLibrary.FinalOverrideCameraArmLengthInterpParams` self CameraParams OutInterpParams))
    (:`then_1`
      (return true))))

(fn `BPOverrideCameraDesiredPivotLocation`
  (params (CurrentCameraPivotLocation :type "Vector Structure") (DesiredCameraPivotLocation :type "Vector Structure (by ref)"))
  (returns (ReturnValue :type Boolean))
  (`|ExecutionSequence`
    (:`then_0`
      (`/Game/PrimalEarth/CoreBlueprints/BPFunctionLibraries/ASACameraFunctionLibrary.FinalOverridePivotLocation` self CurrentCameraPivotLocation DesiredCameraPivotLocation))
    (:`then_1`
      (return true))))

(fn `BPOverrideCameraDesiredPivotOffset`
  (params (CameraParams :type "PrimalCameraParams Structure (by ref)") (DesiredCameraOffset :type "Vector Structure (by ref)"))
  (returns (ReturnValue :type Boolean))
  (`|ExecutionSequence`
    (:`then_0`
      (`/Game/PrimalEarth/CoreBlueprints/BPFunctionLibraries/ASACameraFunctionLibrary.FinalOverridePivotOffset` self CameraParams (`.PitchBasedModifiers` (break `PrimalCameraParams` CameraParams)) DesiredCameraOffset))
    (:`then_1`
      (return true))))

(fn `BPOverrideCameraDesiredPivotRotation`
  (params (CurrentCameraPivotRotation :type "Rotator Structure") (DesiredCameraPivotRotation :type "Rotator Structure (by ref)"))
  (returns (ReturnValue :type Boolean))
  (`|VariableSetRef` DesiredCameraPivotRotation (`KismetMathLibrary.MakeRotator` 0.0 (.pitch DesiredCameraPivotRotation) (.yaw DesiredCameraPivotRotation)))
  (return true))

(fn `BPOverrideCameraPivotLocationInterpParams`
  (params (CameraParams :type "PrimalCameraParams Structure (by ref)") (PivotZInterpOverrides :type "PrimalCameraPivotZInterpOverrides Structure (by ref)") (LastInterpParamsX :type "PrimalCameraInterpParams Structure (by ref)") (LastInterpParamsY :type "PrimalCameraInterpParams Structure (by ref)") (LastInterpParamsZ :type "PrimalCameraInterpParams Structure (by ref)") (OutInterpParamsX :type "PrimalCameraInterpParams Structure (by ref)") (OutInterpParamsY :type "PrimalCameraInterpParams Structure (by ref)") (OutInterpParamsZ :type "PrimalCameraInterpParams Structure (by ref)"))
  (returns (ReturnValue :type Boolean))
  (`|ExecutionSequence`
    (:`then_0`
      (`/Game/PrimalEarth/CoreBlueprints/BPFunctionLibraries/ASACameraFunctionLibrary.Final Override Pivot Interp Params` self CameraParams PivotZInterpOverrides LastInterpParamsX LastInterpParamsY LastInterpParamsZ OutInterpParamsX OutInterpParamsY OutInterpParamsZ))
    (:`then_1`
      (return true))))

(fn `BPTryMultiUse`
  (params (ForPC :type "PlayerController Object Reference") (UseIndex :type Integer))
  (returns (ReturnValue :type Boolean))
  (bind _returnvalue (`parent.BPTryMultiUse` ForPC UseIndex))
  (`|ExecutionSequence`
    (:`then_0`
      (if (and (== UseIndex 111115) (== (`Actor.TargetingTeam` ForPC) (`self.TamingTeamID`)))
        (set `self.SupportsConsumablesAutoTransfer` (not (`self.SupportsConsumablesAutoTransfer`)) true)))
    (:`then_1`
      (return _returnvalue))))

(fn `FearTheManticore`
  (params (ShouldFear :type Boolean)))

(fn `GetDinoContentData`
  (returns (DinoContentData :type "/Game/PrimalEarth/CoreBlueprints/DinoContentData Structure"))
  (return (`self.ContentData`)))

(fn `GetFXBloodColor`
  (returns (ReturnValue :type "LinearColor Structure"))
  (bind _hurtdecaldata_decalmaterial (break `DecalData` (`self.HurtDecalData`)))
  (bind (_lefts _rights _returnvalue) (`KismetStringLibrary.Split` (`KismetSystemLibrary.GetDisplayName` _hurtdecaldata_decalmaterial) "_" "IgnoreCase" "FromEnd"))
  (if _returnvalue
    (switch `string` _rights
      (:`Default`
        _)
      (:`Green`
        (return (struct :`R` 0.105613 :`G` 1.0 :`A` 1.0)))
      (:`Yellow`
        (return (struct :`R` 0.955642 :`G` 1.0 :`B` 0.147486 :`A` 1.0)))
      (:`Bionic`
        (return (struct :`G` 5.705104 :`B` 10.0 :`A` 1.0)))
      (:`Cyan`
        (return (struct :`R` 0.093989 :`G` 0.737358 :`B` 1.0 :`A` 1.0)))
      (:`Corrupted`
        (return (struct :`R` 0.10854 :`G` 0.037732 :`B` 0.242281 :`A` 1.0)))))
  (`parent.GetFXBloodColor`)
  (return (struct :`R` 0.09375 :`B` 0.03 :`A` 1.0)))

(fn `SetSubmarineStructure`
  (params (Structure :type "PrimalStructure Object Reference")))

(fn `UserConstructionScript`)