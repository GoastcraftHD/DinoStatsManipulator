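; Beaver creature Blueprint that spawns a structure, apparently a beaver dam, when an untamed beaver leaves stasis.
; After cooldowns and a short delay, it requires walking or swimming, a biome volume and room under the nearby structure cap.
; It places the structure at a trace hit, then stamps the spawn time on surrounding beavers to throttle further dams.
; The biome tag comparison gates nothing, and the interval variable is unused.
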(event `self.BPUnstasis`
  (bind _returnvalue (`KismetSystemLibrary.GetGameTimeInSeconds` null))
  (bind _returnvalue_2 (`KismetSystemLibrary.GetGameTimeInSeconds` null))
  (bind _returnvalue_3 (`self.K2_GetActorLocation`))
  (bind _structurebiomecustomtagname (`self.StructureBiomeCustomTagName`))
  (bind _unstasisstructuretospawn (`self.UnstasisStructureToSpawn`))
  (bind _movementmode (`CharacterMovementComponent.MovementMode` (`self.CharacterMovement`)))
  (if (`self.BPIsTamed`)
    _
    (elif (> (- _returnvalue (`self.LastUnstasisStructureTime`)) 9000.0)
      (set `self.LastUnstasisStructureTime` _returnvalue)
      (`KismetSystemLibrary.RetriggerableDelay` null 3.0)
      (if (> (- _returnvalue_2 (`self.LastBeaverDamSpawn`)) 9000.0)
        (set `self.LastBeaverDamSpawn` _returnvalue_2)
        (if (and (not (`self.bStasised`)) (or (`|EnumEquality` _movementmode "MOVE_Walking") (`|EnumEquality` _movementmode "MOVE_Swimming")))
          (bind _returnvalue_4 (`BiomeZoneVolume.GetBiomeZoneVolume` (`self.K2_GetWorld`) _returnvalue_3))
          (if (`KismetSystemLibrary.IsValid` _returnvalue_4)
            (if (or (== (`Actor.CustomTag` _returnvalue_4) _structurebiomecustomtagname) (== (`ActorComponent.CustomTag` (`Brush.BrushComponent` _returnvalue_4)) _structurebiomecustomtagname))
              _
              (else
                _))
            (bind _outactors (`KismetSystemLibrary.SphereOverlapActorsSimple` null _returnvalue_3 (`self.StructureCheckRadius`) "ObjectTypeQuery9" _unstasisstructuretospawn))
            (if (< (`KismetArrayLibrary.Array_Length` _outactors) (`self.MaxStructuresInRadius`))
              (bind (_outhit _returnvalue_5) (`KismetSystemLibrary.LineTraceSingle` null _returnvalue_3 (+ _returnvalue_3 (`self.StructureTraceImpactOffset`)) "TraceTypeQuery16"))
              (if _returnvalue_5
                (bind (_bblockinghit _binitialoverlap _time _distance _location) (`GameplayStatics.BreakHitResult` _outhit))
                (`|SpawnActorFromClass` _unstasisstructuretospawn (`KismetMathLibrary.MakeTransform` _location (`self.K2_GetActorRotation`)) "AlwaysSpawn" "SelectDefaultAtRuntime" null null)
                (bind _outactors_2 (`KismetSystemLibrary.SphereOverlapActorsSimple` null _location 50000.0 "ObjectTypeQuery7" "/Game/PrimalEarth/Dinos/Beaver/Beaver_Character_BP.Beaver_Character_BP_C"))
                (for _array_element _outactors_2
                  (bind _asg_beaver_character_bp (cast `/Game/Dinos/G_Beaver_Character_BP` _array_element))
                  (set `/Game/Dinos/G_Beaver_Character_BP.LastBeaverDamSpawn` _returnvalue _asg_beaver_character_bp))))))))))

(fn `UserConstructionScript`
  (`parent.UserConstructionScript`))