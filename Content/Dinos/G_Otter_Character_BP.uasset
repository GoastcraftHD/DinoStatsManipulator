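; Otter dino character that is wake-tamed by feeding it dragged fish and retrieves pearls once tamed.
; Feeding is a timed multi-use entry that converts valid fish into food and team-bound affinity.
; Fish kills trigger a weighted item roll and follow order; a server timer detects owner arrival, rolls a bonus black pearl and multicasts the presentation montage.
; When launched, it sphere-traces the owner's view to force-target an enemy fish.
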(event `self.ReceiveBeginPlay`
  (`parent.ReceiveBeginPlay`)
  (`self.Init`)
  (if (`KismetSystemLibrary.IsDedicatedServer` null)
    (`ActorComponent.K2_DestroyComponent` (`self.pearlMesh`))
    (`ActorComponent.K2_DestroyComponent` (`self.BlackParticle`))
    (`ActorComponent.K2_DestroyComponent` (`self.WhiteParticle`))))

(event `AnimNotify_ShowPearl`
  (bind _pearlmesh (`self.pearlMesh`))
  (bind _whiteparticle (`self.WhiteParticle`))
  (if (not (`KismetSystemLibrary.IsDedicatedServer` null))
    (switch `int` (`self.PearlToShow`)
      (:`1`
        (`PrimitiveComponent.SetMaterial` _pearlmesh 0 "/Game/PrimalEarth/droppedMeshes/BasicResources/Pearl/MIC_OtterPearl.MIC_OtterPearl")
        (`SceneComponent.SetHiddenInGame` _pearlmesh false false true)
        (`ActorComponent.SetActive` _whiteparticle true false)
        (`KismetSystemLibrary.Delay` null 1.4)
        (`SceneComponent.SetHiddenInGame` _pearlmesh true true true)
        (`ActorComponent.SetActive` _whiteparticle false false))
      (:`2`
        (`PrimitiveComponent.SetMaterial` _pearlmesh 0 "/Game/PrimalEarth/droppedMeshes/BasicResources/Pearl/MIC_OtterPearl_Black.MIC_OtterPearl_Black")
        (`SceneComponent.SetHiddenInGame` _pearlmesh false false true)
        (`ActorComponent.SetActive` (`self.BlackParticle`) true false)
        (`KismetSystemLibrary.Delay` null 1.4)
        (`SceneComponent.SetHiddenInGame` _pearlmesh true false true)
        (`ActorComponent.SetActive` (`self.BlackParticle`) false false)))))

(event `MulticastPlayShowPearl`
  (params (switchIndex :type Integer))
  (set `self.PearlToShow` switchIndex)
  (bind _asanim_montage (cast `AnimMontage` (`KismetMathLibrary.SelectObject` "/Game/PrimalEarth/Dinos/Otter/Animations/Otter-Swim-Back-In_Montage.Otter-Swim-Back-In_Montage" "/Game/PrimalEarth/Dinos/Otter/Animations/Otter-Present-Pearl_Montage.Otter-Present-Pearl_Montage" (`|EnumEquality` (`CharacterMovementComponent.MovementMode` (`self.CharacterMovement`)) "MOVE_Swimming"))))
  (`self.PlayAnimEx` _asanim_montage))

(fn `AttemptToGetAPearl`
  (returns (ObtainedAPearl :type Boolean))
  (locals (RetGotPearl :type Boolean))
  (set `local.RetGotPearl` false)
  (`|ExecutionSequence`
    (:`then_0`
      (bind (_gotapearl _indexofselecteditem) (`self.SelectPearl`))
      (if _gotapearl
        (`PrimalItem.AddNewItem` (`|GetArrayItem` (`self.ItemToGive`) _indexofselecteditem) (`self.MyInventoryComponent`) false false 0.0 false 1 false 0.0 false null)
        (set `local.RetGotPearl` true)))
    (:`then_1`
      (return (`local.RetGotPearl`)))))

(fn `BPClientDoMultiUse`
  (params (ForPC :type "PlayerController Object Reference") (ClientUseIndex :type Integer))
  (switch `int` ClientUseIndex
    (:`1667420`
      (bind _asshooter_character (cast `ShooterCharacter` (`Controller.K2_GetPawn` ForPC)))
      (`ShooterWeapon.PlayWeaponAnimation` (`ShooterCharacter.CurrentWeapon` _asshooter_character) (make `WeaponAnim` "/Game/PrimalEarth/HumanMaleFPVHands/Animations/FPV_NoWeapon_Harvesting_Montage.FPV_NoWeapon_Harvesting_Montage") false false false false false false))))

(fn `BPGetMultiUseEntries`
  (params (ForPC :type "PlayerController Object Reference") (MultiUseEntries :type "Array of MultiUseEntry Structure (by ref)"))
  (returns (ReturnValue :type "Array of MultiUseEntry Structure"))
  (bind _wakingtamefeedinterval (`self.WakingTameFeedInterval`))
  (`|ExecutionSequence`
    (:`then_0`
      (bind _asprimal_character (cast `PrimalCharacter` (`Controller.K2_GetPawn` ForPC)))
      (if (`self.BPIsTamed`)
        _
        (elif (or (== (`self.TamingTeamID`) (`Actor.TargetingTeam` _asprimal_character)) (== (`self.TamingTeamID`) 0))
          (bind _asshooter_game_state (cast `ShooterGameState` (`GameplayStatics.GetGameState` null)))
          (bind _returnvalue (`ShooterGameState.GetNetworkTimeDelta` _asshooter_game_state (`self.TimeOfLastFeeding`) false))
          (bind _isvalid (`self.IsCarriedFishValid` _asprimal_character))
          (if (not (`self.IsDead`))
            (bind _returnvalue_2 (`VictoryCore.FormatAsTime` (`KismetMathLibrary.FCeil` (- _wakingtamefeedinterval _returnvalue))))
            (bind _returnvalue_3 (not (>= _returnvalue _wakingtamefeedinterval)))
            (`KismetArrayLibrary.Array_Add` MultiUseEntries (make `MultiUseEntry` null (`KismetMathLibrary.SelectString` (`KismetTextLibrary.Conv_TextToString` (`|FormatText` "Feed Fish {0}" (`KismetTextLibrary.Conv_StringToText` (`KismetMathLibrary.SelectString` (`KismetTextLibrary.Conv_TextToString` (`|FormatText` ": Wait Time {0}" (`KismetTextLibrary.Conv_StringToText` _returnvalue_2))) "" _returnvalue_3)))) "Drag A Fish To Feed" _isvalid) 1667420 1000 false (or _returnvalue_3 (not _isvalid)) false false false false false false false true false false false false null false 0 (make `Color` 200 200 200 200) (make `Color` 40 255 255 255)))))))
    (:`then_1`
      (return MultiUseEntries))))

(fn `BPKilledSomethingEvent`
  (params (killedTarget :type "PrimalCharacter Object Reference"))
  (if (`KismetSystemLibrary.IsServer` null)
    (if (`self.BPIsTamed`)
      (if (not (== (`self.TamedAggressionLevel`) 2))
        (bind _isvalid (`self.IsCharacterAFish` killedTarget))
        (if _isvalid
          (bind _obtainedapearl (`self.AttemptToGetAPearl`))
          (set `self.RecievedAPearl` _obtainedapearl)
          (`self.ReturnToPlayer`))))))

(fn `BPSetupTamed`
  (params (bWasJustTamed :type Boolean))
  (`self.EnableBPTimerServer` true))

(fn `BPTimerServer`
  (switch `int` (`self.CurrentMode`)
    (:`1`
      (`self.Returning To Owner Actions`))))

(fn `BPTryMultiUse`
  (params (ForPC :type "PlayerController Object Reference") (UseIndex :type Integer))
  (returns (ReturnValue :type Boolean))
  (bind _returnvalue (`Controller.K2_GetPawn` ForPC))
  (bind _asprimal_character (cast `PrimalCharacter` _returnvalue))
  (`|ExecutionSequence`
    (:`then_0`
      (switch `int` UseIndex
        (:`1667420`
          (bind _asshooter_character (cast `ShooterCharacter` _returnvalue)
            (:`then`
              (bind _asanim_montage (cast `AnimMontage` (`KismetMathLibrary.SelectObject` "/Game/PrimalEarth/Human/Female/Animations/Female-Pickup_Montage.Female-Pickup_Montage" "/Game/PrimalEarth/Human/Male/Animations/Human-Pickup_Montage.Human-Pickup_Montage" (`ShooterCharacter.bIsFemale` _asshooter_character)))
                (:`then`
                  (`self.PlayAnimEx` _asanim_montage 1.0 "None" true true))
                (:`CastFailed`
                  _)))
            (:`CastFailed`
              _))
          (if (`self.BPIsConscious`)
            (bind _asanim_montage_2 (cast `AnimMontage` (`KismetMathLibrary.SelectObject` "/Game/PrimalEarth/Dinos/Otter/Animations/Otter-Swim-Attack-Bite-Additive_Montage.Otter-Swim-Attack-Bite-Additive_Montage" "/Game/PrimalEarth/Dinos/Otter/Animations/Otter-Eat_Montage.Otter-Eat_Montage" (`|EnumEquality` (`CharacterMovementComponent.MovementMode` (`self.CharacterMovement`)) "MOVE_Swimming")))
              (:`then`
                (`self.PlayAnimEx` _asanim_montage_2 1.0 "None" true true))
              (:`CastFailed`
                _)))
          (`self.EatPlayersCarriedFood` _asprimal_character)
          (set `self.TimeOfLastFeeding` (`KismetSystemLibrary.GetGameTimeInSeconds` null))
          (`self.ForceNetUpdate` false))))
    (:`then_1`
      (return true))))

(fn `EatPlayersCarriedFood`
  (params (Player :type "PrimalCharacter Object Reference"))
  (locals (TamingAmount :type "Float (double-precision)"))
  (bind _tribename (`PrimalCharacter.TribeName` Player))
  (bind _draggedcharacter (`PrimalCharacter.DraggedCharacter` Player))
  (bind _tamingteamid (`self.TamingTeamID`))
  (bind (_isvalid _index) (`self.IsCarriedFishValid` Player))
  (if _isvalid
    (bind _asprimal_dino_character (cast `PrimalDinoCharacter` _draggedcharacter))
    (bind _asshooter_game_mode (cast `ShooterGameMode` (`GameplayStatics.GetGameMode` null)))
    (bind _wildrandomscale (`PrimalDinoCharacter.WildRandomScale` _asprimal_dino_character))
    (set `local.TamingAmount` (* (* (* (- (`self.RequiredTameAffinity`) (* (`PrimalCharacterStatusComponent.BaseCharacterLevel` (`self.MyCharacterStatusComponent`)) (`self.RequiredTameAffinityPerBaseLevel`))) (`|GetArrayItem` (`self.AffinityPercentToGive`) _index)) _wildrandomscale) (`ShooterGameMode.TamingSpeedMultiplier` _asshooter_game_mode)))
    (if (not (`self.BPIsTamed`))
      (`PrimalCharacterStatusComponent.ModifyCurrentStatusValue` (`self.MyCharacterStatusComponent`) "Food" (* (* _wildrandomscale (`PrimalCharacter.DragWeight` _draggedcharacter)) (`self.FoodToGivePerFeeding`)) false false false false null false false)
      (set `self.TameIneffectivenessModifier` (+ (`self.TameIneffectivenessModifier`) (/ (`self.TameIneffectivenessByAffinity`) (`local.TamingAmount`))) true)
      (`|ExecutionSequence`
        (:`then_0`
          (if (== 0 _tamingteamid)
            (set `self.TamingTeamID` (`Actor.TargetingTeam` Player) false)
            (set `self.CurrentTameAffinity` (+ (`self.CurrentTameAffinity`) (`local.TamingAmount`)) false)
            (`self.NetUpdateDinoNameStrings` (`KismetMathLibrary.SelectString` _tribename (`PlayerState.PlayerNamePrivate` (`Pawn.PlayerState` Player)) (> (`KismetStringLibrary.Len` _tribename) 0)))
            (set `self.bIsWakingTame` true false)
            (elif (== (`Actor.TargetingTeam` Player) _tamingteamid)
              (set `self.CurrentTameAffinity` (+ (`self.CurrentTameAffinity`) (`local.TamingAmount`)) false)
              (set `self.bIsWakingTame` true false))))
        (:`then_1`
          (if (>= (`self.CurrentTameAffinity`) (`self.RequiredTameAffinity`))
            (bind _asshooter_game_mode_2 (cast `ShooterGameMode` (`GameplayStatics.GetGameMode` null)))
            (bind _returnvalue (`ShooterGameMode.AllowTaming` _asshooter_game_mode_2 (`self.TamingTeamID`) null))
            (if _returnvalue
              (`self.TameDino` null)
              (switch `EMovementMode` (`CharacterMovementComponent.MovementMode` (`self.CharacterMovement`))
                (:`MOVE_None`
                  _)
                (:`MOVE_Walking`
                  _)
                (:`MOVE_Custom`
                  _))
              (`self.PlayAnimEx` "/Game/PrimalEarth/Dinos/Otter/Animations/Otter-Cuddle_Montage.Otter-Cuddle_Montage" 1.0 "None" true))))
        (:`then_2`
          (`self.K2_DestroyActor` (`PrimalCharacter.DraggedCharacter` Player))
          (`self.EndDragCharacter` Player))))))

(fn `GetOwnerCharacter`
  (returns (Owner :type "Pawn Object Reference"))
  (bind _lastplayertoorder (`self.LastPlayerToOrder`))
  (bind _tamedfollowtarget (`self.TamedFollowTarget`))
  (if (`KismetSystemLibrary.IsServer` null)
    ;[1 1 1] Variable check
    (if (`KismetSystemLibrary.IsValid` _lastplayertoorder)
      (if (not (== (`Actor.TargetingTeam` _lastplayertoorder) (`self.TargetingTeam`)))
        ;[1 1 1] Follow check
        (if (`KismetSystemLibrary.IsValid` _tamedfollowtarget) :!label _label
          (bind _asshooter_character (cast `ShooterCharacter` _tamedfollowtarget)
            (:`then`
              (`self.Set Last Player Order` _asshooter_character))
            (:`CastFailed`
              _))
          (else
            (bind _returnvalue (`VictoryCore.ServerOctreeOverlapActorsClass` null (`self.K2_GetActorLocation`) 5000.0 "PLAYERPAWNS" "/Script/ShooterGame.ShooterCharacter"))
            ;[1 1 1] Overlap check
            (for _array_element _returnvalue
              (bind _asshooter_character_2 (cast `ShooterCharacter` _array_element))
              (`self.Set Last Player Order` _asshooter_character_2)
              (break)))))
      (else
        (goto _label))))
  (return (`self.LastPlayerToOrder`)))

(fn `Init`
  (set `self.TimeOfLastFeeding` -1000.0))

(fn `IsCarriedFishValid`
  (params (Player :type "PrimalCharacter Object Reference"))
  (returns (IsValid :type Boolean) (Index :type Integer))
  (locals (RetValid :type Boolean) (RetIndex :type Integer))
  (bind _draggedcharacter (`PrimalCharacter.DraggedCharacter` Player))
  (set `local.RetIndex` -1)
  (set `local.RetValid` false)
  (`/Engine/EditorBlueprintResources/StandardMacros.IsValid` _draggedcharacter
    (:`Is Valid`
      (for (_array_element _array_index) (`self.ValidTamingClasses`)
        (if (`KismetMathLibrary.ClassIsChildOf` (`GameplayStatics.GetObjectClass` _draggedcharacter) (`|ConvertAsset` _array_element))
          (set `local.RetValid` true)
          (set `local.RetIndex` _array_index))))
    (:`Is Not Valid`
      _))
  (return (`local.RetValid`) (`local.RetIndex`)))

(fn `IsCharacterAFish`
  (params (Character :type "PrimalCharacter Object Reference"))
  (returns (IsValid :type Boolean) (Index :type Integer))
  (locals (RetValid :type Boolean) (RetIndex :type Integer))
  (set `local.RetIndex` -1)
  (set `local.RetValid` false)
  (`/Engine/EditorBlueprintResources/StandardMacros.IsValid` Character
    (:`Is Valid`
      (for (_array_element _array_index) (`self.ValidTamingClasses`)
        (if (`KismetMathLibrary.ClassIsChildOf` (`GameplayStatics.GetObjectClass` Character) (`|ConvertAsset` _array_element))
          (set `local.RetValid` true)
          (set `local.RetIndex` _array_index))))
    (:`Is Not Valid`
      _))
  (return (`local.RetValid`) (`local.RetIndex`)))

(fn `OnLaunched`
  (params (LaunchVelocity :type "Vector Structure") (bXYOverride :type Boolean) (bZOverride :type Boolean))
  (`parent.OnLaunched` LaunchVelocity bXYOverride bZOverride)
  (if (`KismetSystemLibrary.IsServer` null)
    (bind _owner (`self.GetOwnerCharacter`))
    (bind _asshooter_character (cast `ShooterCharacter` _owner))
    (bind (_location _rotation) (`Controller.GetPlayerViewPoint` (`self.GetController` _asshooter_character)))
    (bind _returnvalue (+ _location (* (`KismetMathLibrary.Conv_RotatorToVector` _rotation) 4000.0)))
    ;[1 1 1] Line trace 1 centered
    (`self.ForceUpdateAimedCharacters` (`self.K2_GetWorld`) _location _returnvalue null false 5000.0)
    (bind _outhit (`KismetSystemLibrary.SphereTraceSingleForObjects` null _location _returnvalue (`self.SphereTraceRad`) (`|MakeArray` "ObjectTypeQuery7" :!type "EObjectTypeQuery Enum") false (`|MakeArray` _owner :!type "Actor Object Reference")))
    (bind _asprimal_character (cast `PrimalCharacter` (`.HitActor` (`GameplayStatics.BreakHitResult` _outhit))))
    (bind _isvalid (`self.IsCharacterAFish` _asprimal_character))
    (if _isvalid
      (if (!= (`self.TargetingTeam`) (`Actor.TargetingTeam` _asprimal_character))
        (set `self.ForcedMasterTarget` _asprimal_character)))))

(fn `OnOwnerReached`
  (locals (gotBlackPearl :type Boolean))
  (set `self.CurrentMode` 0)
  (set `local.gotBlackPearl` false)
  (`|ExecutionSequence`
    (:`then_0`
      (if (<= (`KismetMathLibrary.RandomFloatInRange` 0.0 1.0) (`self.ChanceToGiveExtraBlackPearl`))
        (set `local.gotBlackPearl` true)
        (set `self.RecievedAPearl` true)
        (`PrimalItem.AddNewItem` "/Game/PrimalEarth/CoreBlueprints/Resources/PrimalItemResource_BlackPearl.PrimalItemResource_BlackPearl_C" (`self.MyInventoryComponent`) false false 0.0 false 1 false 0.0 false null)))
    (:`then_1`
      (`self.MulticastPlayShowPearl` (`KismetMathLibrary.SelectInt` 2 (`KismetMathLibrary.SelectInt` 1 0 (`self.RecievedAPearl`)) (`local.gotBlackPearl`))))))

(fn `Returning To Owner Actions`
  (if (`KismetSystemLibrary.IsServer` null)
    (if (`self.BPIsTamed`)
      ;[1 1 1] Stop following when owner reached
      (bind _owner (`self.GetOwnerCharacter`))
      (if (<= (`KismetMathLibrary.VSize` (`KismetMathLibrary.MakeVector` (.x (- (`self.K2_GetActorLocation` _owner) (`self.K2_GetActorLocation`))) (.y (- (`self.K2_GetActorLocation` _owner) (`self.K2_GetActorLocation`))))) (`self.BackToOwnerRadius`))
        (`self.OnOwnerReached`)))))

(fn `ReturnToPlayer`
  (if (`KismetSystemLibrary.IsServer` null)
    (if (`self.BPIsTamed`)
      (bind _owner (`self.GetOwnerCharacter`))
      (if (`KismetSystemLibrary.IsValid` _owner)
        (bind _asotter_aicontroller_bp (cast `/Game/PrimalEarth/Dinos/Otter/Otter_AIController_BP` (`self.GetController`)))
        ;[1 1 1] Activate follow
        (bind _asprimal_character (cast `PrimalCharacter` _owner))
        (`self.TamedProcessOrder` _asprimal_character "FollowMe" true null)
        (set `self.CurrentMode` 1)))))

(fn `SelectPearl`
  (returns (GotAPearl :type Boolean) (IndexOfSelectedItem :type Integer))
  (locals (ReturnPearl :type Boolean) (ReturnIndex :type Integer) (`Sum of Weights` :type "Float (double-precision)") (WeightsSoFar :type "Float (double-precision)") (Selector :type "Float (double-precision)"))
  (bind _returnindex (`local.ReturnIndex`))
  (bind _weighttogetitematindex (`self.WeightToGetItemAtIndex`))
  (bind _weightssofar (`local.WeightsSoFar`))
  (set `local.ReturnPearl` false)
  (set `local.ReturnIndex` 0)
  (set `local.Sum of Weights` 0.0)
  (`|ExecutionSequence`
    (:`then_0`
      (for _array_element _weighttogetitematindex
        (set `local.Sum of Weights` (+ _array_element (`local.Sum of Weights`))))
      (set `local.Selector` (`KismetMathLibrary.RandomFloatInRange` 0.0 (`local.Sum of Weights`)))
      (set `local.WeightsSoFar` 0.0)
      (for (_array_element_2 _array_index) _weighttogetitematindex
        (set `local.WeightsSoFar` (+ _array_element_2 _weightssofar))
        (if (<= (`local.Selector`) _weightssofar)
          (set `local.ReturnIndex` _array_index)
          (break))))
    (:`then_1`
      (if (not (== (`|GetArrayItem` (`self.ItemToGive`) _returnindex) null))
        (set `local.ReturnPearl` true)))
    (:`then_2`
      (return (`local.ReturnPearl`) _returnindex))))

(fn `Set Last Player Order`
  (params (Player :type "Pawn Object Reference"))
  (if (`KismetSystemLibrary.IsServer` null)
    (if (`KismetSystemLibrary.IsValid` Player)
      (if (== (`Actor.TargetingTeam` Player) (`self.TargetingTeam`))
        (set `self.LastPlayerToOrder` Player)))))

(fn `UserConstructionScript`
  (`parent.UserConstructionScript`))